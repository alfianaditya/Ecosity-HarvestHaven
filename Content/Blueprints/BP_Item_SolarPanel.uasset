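; Solar panel item Blueprint that builds up an energy total over time.
; Tick feeds a Delay of SpeedTransfer seconds, which acts as a repeating timer because calls made while it is pending are ignored.
; Each time the delay completes, EnergyDefault is added to EnergyGained and the total is printed as debug output.
; Nothing here consumes the energy or checks for sunlight.
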(event EventBeginPlay
  (|CallParentFunction) ; This node is disabled and will not be called.\nDrag off pins to build functionality.
)

(event Collision|EventActorBeginOverlap
  (params (OtherActor :type Actor%20Object%20Reference))
  (|CallParentFunction OtherActor) ; This node is disabled and will not be called.\nDrag off pins to build functionality.
)

(event EventTick
  (params (DeltaSeconds :type Float%20%28single-precision%29))
  (|CallParentFunction DeltaSeconds)
  (Utilities|FlowControl|Delay (Math|Conversions|ToFloat(Integer) (Variables|Default|GetSpeedTransfer)))
  (bind _output_get (Variables|Default|SetEnergyGained (+ (Variables|Default|GetEnergyGained) (Variables|Default|GetEnergyDefault))))
  (Development|PrintString (Utilities|String|ToString(Integer) _output_get)))

(fn ConstructionScript
  (|CallParentFunction))