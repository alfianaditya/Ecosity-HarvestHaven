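; Garden pot actor with three plant slots that the player plants with tomatoes and harvests through a gardening widget.
; Its box overlap toggles input so E opens WBP_Gardening with the mouse cursor and UI-only input.
; Per-slot buttons start Delay-driven mesh swaps through growth stages, then bind harvesting, which only clears the mesh and flags.
; Data-table lookup and item-spawning logic is left disconnected.
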(event OnComponentBeginOverlap(Box)
  (params (OverlappedComponent :type Primitive%20Component%20Object%20Reference) (OtherActor :type Actor%20Object%20Reference) (OtherComp :type Primitive%20Component%20Object%20Reference) (OtherBodyIndex :type Integer) (bFromSweep :type Boolean) (SweepResult :type Hit%20Result%20Structure%20%28by%20ref%29))
  (Utilities|Casting|CastToBP_ThirdPersonCharacter OtherActor)
  (Input|EnableInput (Game|GetPlayerController 0)))

(event OnComponentEndOverlap(Box)
  (params (OverlappedComponent :type Primitive%20Component%20Object%20Reference) (OtherActor :type Actor%20Object%20Reference) (OtherComp :type Primitive%20Component%20Object%20Reference) (OtherBodyIndex :type Integer))
  (Utilities|Casting|CastToBP_ThirdPersonCharacter OtherActor)
  (Input|DisableInput (Game|GetPlayerController 0)))

(event Custom|ButtonPlantA
  (if (Variables|Default|GetPotA)
    (Development|PrintString "SUDAH ADA ISINYA")
    (else
      (Development|PrintString "NANDUR" true true "(R=0.000000,G=0.660000,B=1.000000,A=1.000000)" 1e+01)
      (Components|StaticMesh|SetStaticMesh (Variables|Default|GetPlantA) "/Game/Dummy/tomat1.tomat1")
      (Variables|Default|SetPotA true)
      (Utilities|FlowControl|Delay 5.0)
      (Components|StaticMesh|SetStaticMesh (Variables|Default|GetPlantA) "/Game/Dummy/tomat2.tomat2")
      (Utilities|FlowControl|Delay 5.0)
      (Components|StaticMesh|SetStaticMesh (Variables|Default|GetPlantA) "/Game/Dummy/tomat3.tomat3")
      (Variables|Default|SetPotAReady true)
      (EventDispatchers|BindEventtoOnPressed (Variables|/Game/Inventory/Widgets/WBP_Gardening.WBP_Gardening_C|GetButton_Harvesting_A (Variables|Widget|GetWBP_Garden)) (delegate Custom|HarvestingA)))))

(event Custom|CustomEvent
  (if (Variables|Default|GetPotAReady)
    (Components|StaticMesh|SetStaticMesh (Variables|Default|GetPlantA) 0)
    (Variables|Default|SetPotA false)
    (Variables|Default|SetPotAReady false)))

(event Custom|CustomEvent_3
  (if (Variables|Default|GetPotBReady)
    (Components|StaticMesh|SetStaticMesh (Variables|Default|GetPlantB) 0)
    (Variables|Default|SetPotB false)
    (Variables|Default|SetPotBReady false)))

(event Custom|CustomEvent_1
  (if (Variables|Default|GetPotBReady)
    (Components|StaticMesh|SetStaticMesh (Variables|Default|GetPlantB) 0)
    (Variables|Default|SetPotB false)
    (Variables|Default|SetPotBReady false)))

(event Custom|CustomEvent_2
  (if (Variables|Default|GetPotCReady)
    (Components|StaticMesh|SetStaticMesh (Variables|Default|GetPlantC) 0)
    (Variables|Default|SetPotC false)
    (Variables|Default|SetPotCReady false)))

(event Custom|ButtonPlantB
  (if (Variables|Default|GetPotB)
    (Development|PrintString "SUDAH ADA ISINYA")
    (else
      (Development|PrintString "NANDUR" true true "(R=0.000000,G=0.660000,B=1.000000,A=1.000000)" 1e+01)
      (Components|StaticMesh|SetStaticMesh (Variables|Default|GetPlantB) "/Game/Dummy/tomat1.tomat1")
      (Variables|Default|SetPotB true)
      (Utilities|FlowControl|Delay 5.0)
      (Components|StaticMesh|SetStaticMesh (Variables|Default|GetPlantB) "/Game/Dummy/tomat2.tomat2")
      (Utilities|FlowControl|Delay 5.0)
      (Components|StaticMesh|SetStaticMesh (Variables|Default|GetPlantB) "/Game/Dummy/tomat3.tomat3")
      (Variables|Default|SetPotBReady true)
      (EventDispatchers|BindEventtoOnPressed (Variables|/Game/Inventory/Widgets/WBP_Gardening.WBP_Gardening_C|GetButton_Harvesting_B (Variables|Widget|GetWBP_Garden)) (delegate Custom|CustomEvent_3)))))

(event Custom|ButtonPlantC
  (if (Variables|Default|GetPotC)
    (Development|PrintString "SUDAH ADA ISINYA")
    (else
      (Development|PrintString "NANDUR" true true "(R=0.000000,G=0.660000,B=1.000000,A=1.000000)" 1e+01)
      (Components|StaticMesh|SetStaticMesh (Variables|Default|GetPlantC) "/Game/Dummy/tomat1.tomat1")
      (Variables|Default|SetPotC true)
      (Utilities|FlowControl|Delay 5.0)
      (Components|StaticMesh|SetStaticMesh (Variables|Default|GetPlantC) "/Game/Dummy/tomat2.tomat2")
      (Utilities|FlowControl|Delay 5.0)
      (Components|StaticMesh|SetStaticMesh (Variables|Default|GetPlantC) "/Game/Dummy/tomat3.tomat3")
      (Variables|Default|SetPotCReady true)
      (EventDispatchers|BindEventtoOnPressed (Variables|/Game/Inventory/Widgets/WBP_Gardening.WBP_Gardening_C|GetButton_Harvesting_C (Variables|Widget|GetWBP_Garden)) (delegate Custom|CustomEvent_4)))))

(event Custom|CustomEvent_4
  (if (Variables|Default|GetPotCReady)
    (Components|StaticMesh|SetStaticMesh (Variables|Default|GetPlantC) 0)
    (Variables|Default|SetPotC false)
    (Variables|Default|SetPotCReady false)))

(event Custom|HarvestingA
  (if (Variables|Default|GetPotAReady)
    (Components|StaticMesh|SetStaticMesh (Variables|Default|GetPlantA) 0)
    (Variables|Default|SetPotA false)
    (Variables|Default|SetPotAReady false)))

(event EventBeginPlay
  (|CallParentFunction))

(event Collision|EventActorBeginOverlap
  (params (OtherActor :type Actor%20Object%20Reference))
  (|CallParentFunction OtherActor) ; This node is disabled and will not be called.\nDrag off pins to build functionality.
)

(event EventTick
  (params (DeltaSeconds :type Float%20%28single-precision%29))
  (|CallParentFunction DeltaSeconds) ; This node is disabled and will not be called.\nDrag off pins to build functionality.
)

(event Input|KeyboardEvents|E
  (params (Key :type Key%20Structure :default "None"))
  (bind _returnvalue (Game|GetPlayerController 0))
  (:Pressed
    (Utilities|Casting|CastToBP_ThirdPersonCharacter (stale OnComponentBeginOverlap(Box) OtherActor))
    (Development|PrintString "CEKKK")
    (bind _returnvalue_2 (UserInterface|CreateWidget "/Game/Inventory/Widgets/WBP_Gardening.WBP_Gardening_C"))
    (bind _output_get (Variables|Widget|SetWBP_Garden _returnvalue_2))
    (UserInterface|Viewport|AddtoViewport _output_get 0)
    (Variables|/Script/Engine.PlayerController|SetbShowMouseCursor _returnvalue true)
    (Input|SetInputModeUIOnly _returnvalue (Variables|Widget|GetWBP_Garden) "DoNotLock" false)
    (Utilities|FlowControl|Sequence
      (:then_0
        (Utilities|FlowControl|Sequence
          (:then_0
            (EventDispatchers|BindEventtoOnPressed (Variables|/Game/Inventory/Widgets/WBP_Gardening.WBP_Gardening_C|GetButton_Harvest_A (Variables|Widget|GetWBP_Garden)) (delegate Custom|ButtonPlantA)))
          (:then_1
            (EventDispatchers|BindEventtoOnPressed (Variables|/Game/Inventory/Widgets/WBP_Gardening.WBP_Gardening_C|GetButton_Harvest_B (Variables|Widget|GetWBP_Garden)) (delegate Custom|ButtonPlantB)))
          (:then_2
            (EventDispatchers|BindEventtoOnPressed (Variables|/Game/Inventory/Widgets/WBP_Gardening.WBP_Gardening_C|GetButton_Harvest_C (Variables|Widget|GetWBP_Garden)) (delegate Custom|ButtonPlantC)))))
      (:then_1
        (if (Variables|Default|GetPotAReady)
          (EventDispatchers|BindEventtoOnPressed (Variables|/Game/Inventory/Widgets/WBP_Gardening.WBP_Gardening_C|GetButton_Harvesting_A (Variables|Widget|GetWBP_Garden)) (delegate Custom|CustomEvent))))
      (:then_2
        (if (Variables|Default|GetPotBReady)
          (EventDispatchers|BindEventtoOnPressed (Variables|/Game/Inventory/Widgets/WBP_Gardening.WBP_Gardening_C|GetButton_Harvesting_B (Variables|Widget|GetWBP_Garden)) (delegate Custom|CustomEvent_1))))
      (:then_3
        (if (Variables|Default|GetPotCReady)
          (EventDispatchers|BindEventtoOnPressed (Variables|/Game/Inventory/Widgets/WBP_Gardening.WBP_Gardening_C|GetButton_Harvesting_C (Variables|Widget|GetWBP_Garden)) (delegate Custom|CustomEvent_2)))))))

(fn ConstructionScript
  (|CallParentFunction))